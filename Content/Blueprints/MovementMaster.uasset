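; MovementMaster is a clickable teleport marker that moves the first-person character to its location.
; Clicking its static mesh teleports the player to the marker's X and Y at a fixed height, using the root's relative rotation.
; Tick re-caches the player pawn and, through a short Delay, matches the mesh's visibility to the character's ShowCylinders flag.
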(event `self.ReceiveTick`
  (params (DeltaSeconds :type "Float (single-precision)"))
  (`|ExecutionSequence`
    (:`then_0`
      (`KismetSystemLibrary.Delay` 0.25)
      (if (`/Game/FirstPerson/Blueprints/BP_FirstPersonCharacter.ShowCylinders` (`self.Player`))
        (`SceneComponent.SetVisibility` (`self.StaticMesh`) true false)
        (else
          (`SceneComponent.SetVisibility` (`self.StaticMesh`) false false))))
    (:`then_1`
      (bind _asbp_first_person_character (cast `/Game/FirstPerson/Blueprints/BP_FirstPersonCharacter` (`GameplayStatics.GetPlayerPawn` 0)))
      (set `self.Player` _asbp_first_person_character))))

(event `self.StaticMesh.OnClicked`
  (params (TouchedComponent :type "PrimitiveComponent Object Reference") (ButtonPressed :type "Key Structure"))
  (bind _defaultsceneroot (`self.DefaultSceneRoot`))
  (bind (_returnvalue_x _returnvalue_y) (`KismetMathLibrary.BreakVector` (`SceneComponent.K2_GetComponentLocation` _defaultsceneroot)))
  (`self.K2_SetActorLocationAndRotation` (`self.Player`) (`KismetMathLibrary.MakeVector` _returnvalue_x _returnvalue_y -200.0) (`SceneComponent.RelativeRotation` _defaultsceneroot) false true))

(fn `UserConstructionScript`)
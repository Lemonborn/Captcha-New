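; WrongEnding is a Room 3 Blueprint with a clickable cube that triggers an ending, gated by a Puzzle flag.
; On click with Puzzle true, it fades the camera out over a short delay, then shows the Endong widget.
; Otherwise it shows the Locked widget.
; BeginPlay caches the first-person character, though the click logic does not use it.
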(event `self.ReceiveBeginPlay`
  (bind _asbp_first_person_character (cast `/Game/FirstPerson/Blueprints/BP_FirstPersonCharacter` (`GameplayStatics.GetPlayerPawn` 0)))
  (set `self.Player` _asbp_first_person_character))

(event `self.Cube.OnClicked`
  (params (TouchedComponent :type "PrimitiveComponent Object Reference") (ButtonPressed :type "Key Structure"))
  (if (`self.Puzzle`)
    (`PlayerCameraManager.StartCameraFade` :`self` (`GameplayStatics.GetPlayerCameraManager` 0) :`ToAlpha` 1.0 :`Duration` 2.0)
    (`KismetSystemLibrary.Delay` 2.0)
    (bind _returnvalue (`|CreateWidget` "/Game/Widgets/UI/Endong.Endong_C"))
    (`UserWidget.AddToViewport` _returnvalue 0)
    (else
      (bind _returnvalue_2 (`|CreateWidget` "/Game/Widgets/Pop-Ups/Locked.Locked_C"))
      (`UserWidget.AddToViewport` _returnvalue_2 0))))

(fn `UserConstructionScript`)
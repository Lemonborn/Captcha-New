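; Jigsaw puzzle frame for Room 3 that accepts a matching piece carried by the player.
; On BeginPlay it caches the first-person character and the PuzzleOne piece array from a PuzzlePieceMaster actor.
; Clicking Box_1 while holding a piece compares its Tag to that piece's first tag.
; A match spawns a copy using the piece's rotation and scale, with Back1's relative location as the spawn location.
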(event `self.ReceiveBeginPlay`
  (bind _asbp_first_person_character (cast `/Game/FirstPerson/Blueprints/BP_FirstPersonCharacter` (`GameplayStatics.GetPlayerPawn` 0)))
  (set `self.PlayerRef` _asbp_first_person_character)
  (bind _returnvalue (`GameplayStatics.GetActorOfClass` "/Game/Blueprints/Room_3/PuzzlePieceMaster.PuzzlePieceMaster_C"))
  (set `self.Puzzle One` (`/Game/Blueprints/Room_3/PuzzlePieceMaster.Puzzle_One` _returnvalue)))

(event `self.Box_1.OnClicked`
  (params (TouchedComponent :type "PrimitiveComponent Object Reference") (ButtonPressed :type "Key Structure"))
  (bind _playerref (`self.PlayerRef`))
  (bind _output (`|GetArrayItem` (`self.Puzzle One`) (`/Game/FirstPerson/Blueprints/BP_FirstPersonCharacter.PieceID` _playerref)))
  (if (`/Game/FirstPerson/Blueprints/BP_FirstPersonCharacter.PieceHeld?` _playerref)
    (if (== (`self.Tag`) (`|GetArrayItem` (`Actor.Tags` _output)))
      (`|SpawnActorFromClass` (`GameplayStatics.GetObjectClass` _output) (`KismetMathLibrary.MakeTransform` (`SceneComponent.RelativeLocation` (`self.Back_1`)) (`self.K2_GetActorRotation` _output) (`self.GetActorRelativeScale3D` _output)) "AlwaysSpawn" "MultiplyWithRoot" null null))))

(fn `UserConstructionScript`)
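; Puzzle_1_1 is a clickable puzzle piece actor in Room 3 that reports its identity to the player when selected.
; Clicking its static mesh while the player already holds a piece shows a PieceHeld widget.
; Otherwise it looks up its own index in the PuzzleOne array, debug-prints it and stores it as the player's PieceID.
; PlayerRef and PuzzleOne are not assigned in these graphs.
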(event `self.StaticMesh.OnClicked`
  (params (TouchedComponent :type "PrimitiveComponent Object Reference") (ButtonPressed :type "Key Structure"))
  (bind _returnvalue (`KismetArrayLibrary.Array_Find` (`self.Puzzle_One`) self))
  (if (`/Game/FirstPerson/Blueprints/BP_FirstPersonCharacter.PieceHeld?` (`self.PlayerRef`))
    (bind _returnvalue_2 (`|CreateWidget` "/Game/Widgets/Pop-Ups/PieceHeld.PieceHeld_C"))
    (`UserWidget.AddToViewport` _returnvalue_2 0)
    (else
      (`KismetSystemLibrary.PrintString` (`KismetStringLibrary.Conv_IntToString` _returnvalue))
      (set `/Game/FirstPerson/Blueprints/BP_FirstPersonCharacter.PieceID` _returnvalue (`self.PlayerRef`)))))

(fn `UserConstructionScript`
  (`parent.UserConstructionScript`))
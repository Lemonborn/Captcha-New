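; Master Blueprint for an inspectable item that lets the player spin its static mesh with the mouse.
; While the middle mouse button is held, MouseX axis input adds roll and MouseY adds pitch to the mesh's relative rotation.
; Each axis value is negated and merged through CombineRotators.
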(event `InputAxisKey|MouseX`
  (params (AxisValue :type "Float (single-precision)"))
  (if (`PlayerController.IsInputKeyDown` (`GameplayStatics.GetPlayerController` 0) "MiddleMouseButton")
    (`SceneComponent.K2_SetRelativeRotation` (`self.StaticMesh`) (`KismetMathLibrary.ComposeRotators` (`SceneComponent.RelativeRotation` (`self.StaticMesh`)) (`KismetMathLibrary.MakeRotator` (* AxisValue -1.0))) false false)))

(event `InputAxisKey|MouseY`
  (params (AxisValue :type "Float (single-precision)"))
  (if (`PlayerController.IsInputKeyDown` (`GameplayStatics.GetPlayerController` 0) "MiddleMouseButton")
    (`SceneComponent.K2_SetRelativeRotation` (`self.StaticMesh`) (`KismetMathLibrary.ComposeRotators` (`SceneComponent.RelativeRotation` (`self.StaticMesh`)) (`KismetMathLibrary.MakeRotator` 0.0 (* AxisValue -1.0))) false false)))

(fn `UserConstructionScript`)
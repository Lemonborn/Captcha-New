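; PickupMaster is a pickup Blueprint, apparently a base class, that lets the first-person player collect an item only once it is revealed.
; BeginPlay caches the player's BP_FirstPersonCharacter.
; When revealed, PickUp sets the Item flag, shows an optional widget if one is assigned and passes the instigating argument to the character's Pickup.
; Otherwise it shows the Missing widget and clears the flag.
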(event `self.ReceiveBeginPlay`
  (bind _asbp_first_person_character (cast `/Game/FirstPerson/Blueprints/BP_FirstPersonCharacter` (`GameplayStatics.GetPlayerPawn` 0))
    (:`then`
      (set `self.Player` _asbp_first_person_character))
    (:`CastFailed`
      (`KismetSystemLibrary.PrintString` "Hello"))))

(event `PickUp`
  (params (Instigating :type "Actor Object Reference"))
  (if (`self.Revealed`)
    (if (`self.Widget?`)
      (set `self.Item` true)
      (bind _returnvalue (`|CreateWidget` (`self.Widget`) (`GameplayStatics.GetPlayerController` 0)))
      (`UserWidget.AddToViewport` _returnvalue 0)
      (`/Game/FirstPerson/Blueprints/BP_FirstPersonCharacter.Pickup` (`self.Player`) Instigating)
      (else
        (set `self.Item` true)
        (`/Game/FirstPerson/Blueprints/BP_FirstPersonCharacter.Pickup` (`self.Player`) Instigating)))
    (else
      (bind _returnvalue_2 (`|CreateWidget` "/Game/Widgets/Pop-Ups/Missing.Missing_C" (`GameplayStatics.GetPlayerController` 0)))
      (`UserWidget.AddToViewport` _returnvalue_2 0)
      (set `self.Item` false))))

(fn `UserConstructionScript`)
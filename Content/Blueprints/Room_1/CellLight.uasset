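; CellLight is a Room 1 point-light actor that lights the cell based on the player's state.
; At BeginPlay it caches the first-person character and turns the light off.
; Each Tick it sets the light to a fixed intensity while the player's Movement flag is set and the jigsaw is not done.
; Nothing here switches the light back off afterward.
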(event `self.ReceiveBeginPlay`
  (bind _asbp_first_person_character (cast `/Game/FirstPerson/Blueprints/BP_FirstPersonCharacter` (`GameplayStatics.GetPlayerPawn` 0)))
  (set `self.PlayerRef` _asbp_first_person_character)
  (`LightComponent.SetIntensity` (`self.PointLightComponent`) 0.0))

(event `self.ReceiveTick`
  (params (DeltaSeconds :type "Float (single-precision)"))
  (bind _playerref (`self.PlayerRef`))
  (if (and (`/Game/FirstPerson/Blueprints/BP_FirstPersonCharacter.Movement` _playerref) (not (`/Game/FirstPerson/Blueprints/BP_FirstPersonCharacter.JigsawDone?` _playerref)))
    (`LightComponent.SetIntensity` (`self.PointLightComponent`) 100.0)))

(fn `UserConstructionScript`)
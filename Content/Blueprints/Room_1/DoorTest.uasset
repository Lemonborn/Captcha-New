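; DoorTest is a Room 1 Blueprint with a clickable cube that operates a door once the player's DeadRat flag is true.
; A click casts the first actor tagged "Door" to DoorMaster and copies the flag into its Locked variable, where true means passable.
; If true, a FlipFlop alternates CharacterLocation between two fixed points before calling OpenDoor.
; Otherwise, it shows a Locked widget.
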(event `self.Cube.OnClicked`
  (params (TouchedComponent :type "PrimitiveComponent Object Reference") (ButtonPressed :type "Key Structure"))
  (bind _outactors (`GameplayStatics.GetAllActorsWithTag` "Door"))
  (bind _asdoor_master (cast `/Game/Blueprints/DoorMaster` (`|GetArrayItem` _outactors)))
  (bind _output_get (set `/Game/Blueprints/DoorMaster.Locked` (`/Game/FirstPerson/Blueprints/BP_FirstPersonCharacter.DeadRat` (`/Game/Blueprints/DoorMaster.Player` _asdoor_master)) _asdoor_master))
  (if _output_get
    (`/Engine/EditorBlueprintResources/StandardMacros.FlipFlop`
      (:`A`
        (set `/Game/Blueprints/DoorMaster.CharacterLocation` (870.0 1730.0 82.0) _asdoor_master))
      (:`B`
        (set `/Game/Blueprints/DoorMaster.CharacterLocation` (870.0 1230.0 82.0) _asdoor_master)))
    (`self.OpenDoor` _asdoor_master)
    (else
      (bind _returnvalue (`|CreateWidget` "/Game/Widgets/Pop-Ups/Locked.Locked_C"))
      (`UserWidget.AddToViewport` _returnvalue 0))))

(fn `UserConstructionScript`
  (`parent.UserConstructionScript`))
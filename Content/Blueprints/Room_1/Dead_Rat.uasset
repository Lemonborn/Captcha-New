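; Dead Rat is a clickable pickup in Room 1 that the player can collect.
; Clicking its mesh finds the first Pickup-tagged PickupMaster, copies the player's Brick flag into its Revealed state, sets the Rat widget and calls PickUp.
; If the master's Item flag is then true, it sets the player's DeadRat flag and destroys itself.
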(event `self.StaticMesh.OnClicked`
  (params (TouchedComponent :type "PrimitiveComponent Object Reference") (ButtonPressed :type "Key Structure"))
  (bind _outactors (`GameplayStatics.GetAllActorsWithTag` "Pickup"))
  (bind _aspickup_master (cast `/Game/Blueprints/PickupMaster` (`|GetArrayItem` _outactors)))
  (set `/Game/Blueprints/PickupMaster.Revealed` (`/Game/FirstPerson/Blueprints/BP_FirstPersonCharacter.Brick` (`/Game/Blueprints/PickupMaster.Player` _aspickup_master)) _aspickup_master)
  (set `/Game/Blueprints/PickupMaster.Widget` "/Game/Widgets/Pop-Ups/Rat.Rat_C" _aspickup_master)
  (`self.PickUp` _aspickup_master null)
  (if (`/Game/Blueprints/PickupMaster.Item` _aspickup_master)
    (set `/Game/FirstPerson/Blueprints/BP_FirstPersonCharacter.DeadRat` true (`/Game/Blueprints/PickupMaster.Player` _aspickup_master))
    (`self.K2_DestroyActor`)))

(fn `UserConstructionScript`
  (`parent.UserConstructionScript`))
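; Clickable destructible brick for Room 1 that breaks only when the player holds the Bone item.
; On BeginPlay it stores the class of a Brick actor found in the level, its own mesh location and rotation, and that Brick's scale.
; Clicking the mesh compares the player's ItemActor with the level's Bone actor.
; A match calls Break, defined outside this graph; otherwise a Missing widget appears on screen.
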(event `self.ReceiveBeginPlay`
  (bind _staticmesh (`self.StaticMesh`))
  (bind _returnvalue (`GameplayStatics.GetActorOfClass` "/Game/Blueprints/Room_1/brick.brick_C"))
  (set `self.Class` (`GameplayStatics.GetObjectClass` _returnvalue))
  (`|ExecutionSequence`
    (:`then_0`
      (set `self.Location` (`SceneComponent.K2_GetComponentLocation` _staticmesh)))
    (:`then_1`
      (set `self.Rotation` (`SceneComponent.K2_GetComponentRotation` _staticmesh)))
    (:`then_2`
      (set `self.Scale` (`SceneComponent.K2_GetComponentScale` (`/Game/Blueprints/PickupMaster.StaticMesh` _returnvalue))))))

(event `self.StaticMesh.OnClicked`
  (params (TouchedComponent :type "PrimitiveComponent Object Reference") (ButtonPressed :type "Key Structure"))
  (bind _returnvalue (`GameplayStatics.GetActorOfClass` "/Game/Blueprints/Room_1/Bone.Bone_C"))
  (if (== _returnvalue (`/Game/FirstPerson/Blueprints/BP_FirstPersonCharacter.ItemActor` (`self.Player`)))
    (`self.Break`)
    (else
      (bind _returnvalue_2 (`|CreateWidget` "/Game/Widgets/Pop-Ups/Missing.Missing_C"))
      (`UserWidget.AddToViewport` _returnvalue_2 0))))

(fn `UserConstructionScript`
  (`parent.UserConstructionScript`))
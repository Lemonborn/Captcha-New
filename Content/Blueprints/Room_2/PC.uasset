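; Room 2 PC actor that shows the player the current riddle screen in a chain of puzzles.
; Clicking the mesh or calling UpdateScreen checks the Puzzle, Puzzle2 and Puzzle3 flags in nested order.
; It then creates and adds the matching riddle widget to the viewport, or the PCFinal widget once all three are set.
; BeginPlay clears Puzzle and Puzzle2, but not Puzzle3.
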(event `self.ReceiveBeginPlay`
  (set `self.Puzzle` false)
  (set `self.Puzzle 2` false))

(event `UpdateScreen`
  (if (`self.Puzzle`) :!label _label
    (if (`self.Puzzle 2`)
      (if (`self.Puzzle 3`)
        (bind _returnvalue (`|CreateWidget` "/Game/Widgets/Room_Two/PCFinal.PCFinal_C"))
        (`UserWidget.AddToViewport` _returnvalue 0)
        (else
          (bind _returnvalue_2 (`|CreateWidget` "/Game/Widgets/Room_Two/Riddle3.Riddle3_C"))
          (`UserWidget.AddToViewport` _returnvalue_2 0)))
      (else
        (bind _returnvalue_3 (`|CreateWidget` "/Game/Widgets/Room_Two/Riddle2.Riddle2_C"))
        (`UserWidget.AddToViewport` _returnvalue_3 0)))
    (else
      (bind _returnvalue_4 (`|CreateWidget` "/Game/Widgets/Room_Two/Riddle.Riddle_C"))
      (`UserWidget.AddToViewport` _returnvalue_4 0))))

(event `self.StaticMesh.OnClicked`
  (params (TouchedComponent :type "PrimitiveComponent Object Reference") (ButtonPressed :type "Key Structure"))
  (goto _label))

(fn `UserConstructionScript`)
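; Apple interactable for Room 2 that swaps between two static meshes and sends the player to a fixed spot when clicked.
; Clicking the main mesh teleports the cached first-person character, enables its Movement flag, then after a delay shows the second mesh and sets Done.
; Right mouse hands possession back to the character and restores the main mesh.
; The custom Unpossess event only swaps mesh visibility.
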(event `self.Unpossess`
  (`SceneComponent.SetVisibility` (`self.StaticMesh`) false false)
  (`SceneComponent.SetVisibility` (`self.StaticMesh1`) true false))

(event `Moveplayer`
  (if true
    (`self.K2_SetActorLocationAndRotation` (`self.PlayerRef`) (-500.0 2930.0 -200.0) (struct :`Yaw` 180.0) false true)))

(event `self.StaticMesh.OnClicked`
  (params (TouchedComponent :type "PrimitiveComponent Object Reference") (ButtonPressed :type "Key Structure"))
  (`self.Moveplayer`)
  (set `/Game/FirstPerson/Blueprints/BP_FirstPersonCharacter.Movement` true (`self.PlayerRef`))
  (`KismetSystemLibrary.Delay` 1.0)
  (`SceneComponent.SetVisibility` (`self.StaticMesh`) false false)
  (`SceneComponent.SetVisibility` (`self.StaticMesh1`) true false)
  (set `self.Done` true)
  (`KismetSystemLibrary.Delay` 3.0)
  (`self.Unpossess`))

(event `self.ReceiveBeginPlay`
  (`parent.ReceiveBeginPlay`)
  (set `self.Done` false)
  (bind _returnvalue (`GameplayStatics.GetActorOfClass` "/Game/FirstPerson/Blueprints/BP_FirstPersonCharacter.BP_FirstPersonCharacter_C"))
  (set `self.PlayerRef` _returnvalue))

(event `Apple`
  (`SceneComponent.SetVisibility` (`self.StaticMesh`) true false)
  (`SceneComponent.SetVisibility` (`self.StaticMesh1`) false false))

(event `Key|RightMouseButton`
  (params (Key :type "Key Structure"))
  (bind _returnvalue (`GameplayStatics.GetPlayerController` 0))
  (:`Pressed`
    (`self.Unpossess`)
    (`Controller.UnPossess` _returnvalue)
    (`Controller.Possess` _returnvalue (`self.PlayerRef`))
    (`self.Apple`)))

(fn `UserConstructionScript`
  (`parent.UserConstructionScript`))
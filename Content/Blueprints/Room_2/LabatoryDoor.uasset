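; Laboratory door Blueprint in Room 2 that responds to clicks on its Cube by either opening the way through or triggering an ending.
; It finds the first "Door"-tagged DoorMaster and copies the player's EyeScanned flag into its Locked variable.
; The WrongEnding actor's Puzzle flag then decides between calling the player's Ending and setting a fixed CharacterLocation before calling OpenDoor on the DoorMaster.
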(event `self.Cube.OnClicked`
  (params (TouchedComponent :type "PrimitiveComponent Object Reference") (ButtonPressed :type "Key Structure"))
  (bind _outactors (`GameplayStatics.GetAllActorsWithTag` "Door"))
  (bind _asdoor_master (cast `/Game/Blueprints/DoorMaster` (`|GetArrayItem` _outactors)))
  (bind _player (`/Game/Blueprints/DoorMaster.Player` _asdoor_master))
  (set `/Game/Blueprints/DoorMaster.Locked` (`/Game/FirstPerson/Blueprints/BP_FirstPersonCharacter.EyeScanned` _player) _asdoor_master)
  (bind _returnvalue (`GameplayStatics.GetActorOfClass` "/Game/Blueprints/Room_3/WrongEnding.WrongEnding_C"))
  (if (`/Game/Blueprints/Room_3/WrongEnding.Puzzle` _returnvalue)
    (`/Game/FirstPerson/Blueprints/BP_FirstPersonCharacter.Ending` _player)
    (else
      (set `/Game/Blueprints/DoorMaster.CharacterLocation` (1300.0 2972.0 140.0) _asdoor_master)
      (`self.OpenDoor` _asdoor_master))))

(fn `UserConstructionScript`
  (`parent.UserConstructionScript`))
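; Room_2_Audio is an audio actor Blueprint for Room 2 that exposes events to control its sound playback.
; GameStart starts the AudioComponent, while Pause and Play toggle its paused state.
; Move looks up the Jigsaw_1 actor by class and teleports the audio actor to a fixed X offset from it with a set rotation.
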(event `Game Start`
  (`FMODAudioComponent.Play` (`self.AudioComponent`)))

(event `Pause`
  (`FMODAudioComponent.SetPaused` (`self.AudioComponent`) true))

(event `Play`
  (`FMODAudioComponent.SetPaused` (`self.AudioComponent`) false))

(event `Move`
  (bind _returnvalue (`GameplayStatics.GetActorOfClass` "/Game/Blueprints/Room_3/Jigsaw/Jigsaw_1.Jigsaw_1_C"))
  (bind (_returnvalue_x _returnvalue_y _returnvalue_z) (`KismetMathLibrary.BreakVector` (`self.K2_GetActorLocation` _returnvalue)))
  (`self.K2_SetActorLocationAndRotation` (`KismetMathLibrary.MakeVector` (- _returnvalue_x 500.0) _returnvalue_y _returnvalue_z) (struct :`Yaw` 90.0) false true))

(fn `UserConstructionScript`)
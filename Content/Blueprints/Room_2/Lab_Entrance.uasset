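; Clickable lab entrance door in Room 2 that opens only when the player's DeadRat flag is set.
; On click, it copies that flag into DoorMaster's Locked (true means open), sets CharacterLocation beside DoorTest, and calls OpenDoor.
; It then plays Room 1 audio and pauses Room 2's; otherwise it shows a Locked widget.
; Hovering the cube switches the cursor to a grab hand.
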(event `self.Cube.OnClicked`
  (params (TouchedComponent :type "PrimitiveComponent Object Reference") (ButtonPressed :type "Key Structure"))
  (bind _returnvalue (`GameplayStatics.GetActorOfClass` "/Game/Blueprints/DoorMaster.DoorMaster_C"))
  (bind _output_get (set `/Game/Blueprints/DoorMaster.Locked` (`/Game/FirstPerson/Blueprints/BP_FirstPersonCharacter.DeadRat` (`/Game/Blueprints/DoorMaster.Player` _returnvalue)) _returnvalue))
  (if _output_get
    (bind _returnvalue_2 (`GameplayStatics.GetActorOfClass` "/Game/Blueprints/Room_1/DoorTest.DoorTest_C"))
    (bind (_returnvalue_x _returnvalue_y _returnvalue_z) (`KismetMathLibrary.BreakVector` (`self.K2_GetActorLocation` _returnvalue_2)))
    (set `/Game/Blueprints/DoorMaster.CharacterLocation` (`KismetMathLibrary.MakeVector` _returnvalue_x (- _returnvalue_y 200.0) _returnvalue_z) _returnvalue)
    (`self.OpenDoor` _returnvalue)
    (`|ExecutionSequence`
      (:`then_0`
        (bind _returnvalue_3 (`GameplayStatics.GetActorOfClass` "/Game/Blueprints/Room_1/Room_1_Audio.Room_1_Audio_C"))
        (`/Game/Blueprints/Room_1/Room_1_Audio.Play` _returnvalue_3))
      (:`then_1`
        (bind _returnvalue_4 (`GameplayStatics.GetActorOfClass` "/Game/Blueprints/Room_2/Room_2_Audio.Room_2_Audio_C"))
        (`/Game/Blueprints/Room_2/Room_2_Audio.Pause` _returnvalue_4)))
    (else
      (bind _returnvalue_5 (`|CreateWidget` "/Game/Widgets/Pop-Ups/Locked.Locked_C"))
      (`UserWidget.AddToViewport` _returnvalue_5 0))))

(event `self.Cube.OnBeginCursorOver`
  (params (TouchedComponent :type "PrimitiveComponent Object Reference"))
  (set `PlayerController.CurrentMouseCursor` "GrabHand" (`GameplayStatics.GetPlayerController` 0)))

(event `self.Cube.OnEndCursorOver`
  (params (TouchedComponent :type "PrimitiveComponent Object Reference"))
  (set `PlayerController.CurrentMouseCursor` "Default" (`GameplayStatics.GetPlayerController` 0)))

(fn `UserConstructionScript`
  (`parent.UserConstructionScript`))
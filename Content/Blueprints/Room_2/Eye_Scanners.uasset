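; Eye scanner puzzle object in Room 2 that records a successful eye scan on the player.
; Clicking its mesh looks up The_Machine and, if its Body value is true, swaps the Fail display for Success and sets EyeScanned on Player.
; Pressing Inspect returns controller possession to Player, exiting the scanner.
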(event `self.ReceiveBeginPlay`
  (`parent.ReceiveBeginPlay`))

(event `InputAction|Inspect`
  (params (Key :type "Key Structure"))
  (bind _returnvalue (`GameplayStatics.GetPlayerController` 0))
  (:`Pressed`
    (`Controller.UnPossess` _returnvalue)
    (`Controller.Possess` _returnvalue (`self.Player`))))

(event `self.StaticMesh.OnClicked`
  (params (TouchedComponent :type "PrimitiveComponent Object Reference") (ButtonPressed :type "Key Structure"))
  (bind _returnvalue (`GameplayStatics.GetActorOfClass` "/Game/Blueprints/The_Machine.The_Machine_C"))
  (if (`/Game/Blueprints/The_Machine.Body` _returnvalue)
    (`SceneComponent.SetVisibility` (`self.Fail`) false false)
    (`SceneComponent.SetVisibility` (`self.Success`) true false)
    (set `/Game/FirstPerson/Blueprints/BP_FirstPersonCharacter.EyeScanned` true (`self.Player`))))

(fn `UserConstructionScript`
  (`parent.UserConstructionScript`))
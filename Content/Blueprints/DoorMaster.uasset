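; DoorMaster is a door Blueprint that moves the player to a set destination when opened.
; On BeginPlay it caches the player pawn as a BP_FirstPersonCharacter.
; OpenDoor teleports that character to a stored location and rotation when the Locked flag is true, and otherwise adds a Locked widget to the viewport, so the flag reads inverted relative to its name.
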(event `self.ReceiveBeginPlay`
  (bind _asbp_first_person_character (cast `/Game/FirstPerson/Blueprints/BP_FirstPersonCharacter` (`GameplayStatics.GetPlayerPawn` 0)))
  (set `self.Player` _asbp_first_person_character))

(event `OpenDoor`
  (if (`self.Locked`)
    (`self.K2_SetActorLocationAndRotation` (`self.Player`) (`self.CharacterLocation`) (`self.CharacterRotation`) false true)
    (else
      (bind _returnvalue (`|CreateWidget` "/Game/Widgets/Pop-Ups/Locked.Locked_C"))
      (`UserWidget.AddToViewport` _returnvalue 0))))

(fn `UserConstructionScript`)
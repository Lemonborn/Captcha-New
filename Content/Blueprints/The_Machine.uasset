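; The Machine is a clickable puzzle station that gives the first-person player a body once its requirements are met.
; Clicks check for the bone key, show a one-time genetic error, then check code input and a corpse flag polled from the player, opening matching widgets.
; Success, or a direct Update call, runs once to show the player mesh, teleport the player and update a ReadableMaster actor.
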(event `self.ReceiveTick`
  (params (DeltaSeconds :type "Float (single-precision)"))
  (`KismetSystemLibrary.Delay` 0.2)
  (set `self.Corpse` (`/Game/FirstPerson/Blueprints/BP_FirstPersonCharacter.Corpse` (`self.Player`))))

(event `Update`
  (`/Engine/EditorBlueprintResources/StandardMacros.DoOnce` false :!label _label
    (:`Completed`
      (bind _returnvalue (`|CreateWidget` "/Game/Widgets/Room_Two/GettingBody.GettingBody_C"))
      (`UserWidget.AddToViewport` _returnvalue 0)
      (set `self.Done` true)
      (`SceneComponent.SetVisibility` (`Character.Mesh` (`self.Player`)) true false)
      (`self.K2_SetActorLocationAndRotation` (`self.Player`) (1320.0 2370.0 82.0) (struct :`Yaw` 90.0) false true)
      (bind _returnvalue_2 (`GameplayStatics.GetActorOfClass` "/Game/Blueprints/ReadableMaster.ReadableMaster_C"))
      (`/Game/Blueprints/ReadableMaster.Update` _returnvalue_2))))

(event `self.ReceiveBeginPlay`
  (bind _asbp_first_person_character (cast `/Game/FirstPerson/Blueprints/BP_FirstPersonCharacter` (`GameplayStatics.GetPlayerPawn` 0)))
  (set `self.Player` _asbp_first_person_character)
  (set `self.DoneOnce` false)
  (set `self.Done` false))

(event `self.StaticMesh.OnClicked`
  (params (TouchedComponent :type "PrimitiveComponent Object Reference") (ButtonPressed :type "Key Structure"))
  (bind _player (`self.Player`))
  (set `/Game/FirstPerson/Blueprints/BP_FirstPersonCharacter.BioMachine` false _player)
  (if (`/Game/FirstPerson/Blueprints/BP_FirstPersonCharacter.BoneKey` _player)
    (`|ExecutionSequence`
      (:`then_0`
        (`/Engine/EditorBlueprintResources/StandardMacros.DoOnce` false
          (:`Completed`
            (bind _returnvalue (`|CreateWidget` "/Game/Widgets/Room_Two/GeneticERROR.GeneticERROR_C"))
            (`UserWidget.AddToViewport` _returnvalue 0)
            (`KismetSystemLibrary.Delay` 3.0)
            (set `self.DoneOnce` true)
            (if (`self.CodeInput`) :!label _label_2
              (if (`self.Corpse`)
                (goto _label)
                (else
                  (bind _returnvalue_2 (`|CreateWidget` "/Game/Widgets/Pop-Ups/Missing.Missing_C"))
                  (`UserWidget.AddToViewport` _returnvalue_2 0)))
              (else
                (bind _returnvalue_3 (`|CreateWidget` "/Game/Widgets/Room_Two/MachineCode.MachineCode_C"))
                (`UserWidget.AddToViewport` _returnvalue_3 0))))))
      (:`then_1`
        (if (`self.DoneOnce`)
          (goto _label_2))))
    (else
      (bind _returnvalue_4 (`|CreateWidget` "/Game/Widgets/Pop-Ups/KeyRequired.KeyRequired_C"))
      (`UserWidget.AddToViewport` _returnvalue_4 0))))

(fn `UserConstructionScript`)
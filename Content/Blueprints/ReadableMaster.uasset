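; ReadableMaster is a possessable base Blueprint, apparently for readable objects the player inspects.
; Clicking its static mesh makes the player controller possess it.
; The Inspect input or the Unpossess event returns control to the BP_FirstPersonCharacter reference cached on BeginPlay or Update.
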(event `Update`
  (bind _asbp_first_person_character (cast `/Game/FirstPerson/Blueprints/BP_FirstPersonCharacter` (`GameplayStatics.GetPlayerCharacter` 0) :!label _label))
  (set `self.Player` _asbp_first_person_character))

(event `self.StaticMesh.OnClicked`
  (params (TouchedComponent :type "PrimitiveComponent Object Reference") (ButtonPressed :type "Key Structure"))
  (`Controller.Possess` (`GameplayStatics.GetPlayerController` 0) self))

(event `self.ReceiveBeginPlay`
  (goto _label))

(event `InputAction|Inspect`
  (params (Key :type "Key Structure"))
  (bind _returnvalue (`GameplayStatics.GetPlayerController` 0))
  (:`Pressed`
    (`Controller.UnPossess` _returnvalue :!label _label_2)
    (`Controller.Possess` _returnvalue (`self.Player`))))

(event `Unpossess`
  (goto _label_2))

(fn `UserConstructionScript`)